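; GM_BeginGame is a game mode that registers joining players and spawns a Basic_Pawn for each to possess.
; On the first authority login, PostLogin caches all PlayerStarts; every login stores the controller and calls REspawnPlayerEvent.
; That event destroys any existing pawn, then spawns and possesses a new one at a random start.
; Debug-gated logging traces the flow, but separate random rolls mean logged spawn points can differ from the one used.
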(event `self.K2_PostLogin`
  (params (NewPlayer :type "PlayerController Object Reference"))
  (bind _asmy_player_controller (cast `/Game/BeginGame/GameMode/MyPlayerController` NewPlayer))
  (`/Engine/EditorBlueprintResources/ActorMacros.Switch Has Authority`
    (:`Authority`
      (`self.OutputLog` "OnPostLogin Start")
      ;[1 1 1] Initial Setup Find all the Player Starts
      (if (`self.InitialSetupDone?`)
        (`self.OutputLog` "PostLogin No Setup Required")
        (else
          (set `self.InitialSetupInProgress` true)
          (`self.OutputLog` "Run Initial Setup")
          (bind _outactors (`GameplayStatics.GetAllActorsOfClass` "/Script/Engine.PlayerStart"))
          (for _array_element _outactors
            (`KismetArrayLibrary.Array_AddUnique` (`self.SpawnPointsFullList`) _array_element)
            (set `self.InitialSetupDone?` true)
            (bind _output_get (set `self.NumberSpawnPoints` (`KismetArrayLibrary.Array_Length` (`self.SpawnPointsFullList`))))
            (`self.OutputLog` "Number Pawns : " (`KismetTextLibrary.Conv_IntToText` _output_get))))))
    (:`Remote`
      _))
  ;[1 1 1] Join the New Player to the Game and Start the Client Login Process
  (`KismetArrayLibrary.Array_AddUnique` (`self.PlayerControllerRefs`) _asmy_player_controller)
  (`self.ClientNumber` _asmy_player_controller)
  (`self.REspawnPlayerEvent` _asmy_player_controller))

(event `REspawnPlayerEvent`
  (params (MyPlayerController :type "/Game/BeginGame/GameMode/MyPlayerController Object Reference"))
  (bind _returnvalue (`Controller.K2_GetPawn` MyPlayerController))
  (bind _returnvalue_2 (`KismetMathLibrary.RandomInteger` (`self.NumberSpawnPoints`)))
  (bind _returnvalue_3 (`self.GetTransform` (`KismetArrayLibrary.Array_Get` (`self.SpawnPointsFullList`) _returnvalue_2)))
  (`/Game/BeginGame/GameMode/MyPlayerController.Outputlog` MyPlayerController "*Inside gm respawnplayerevent" "")
  ;[0.2847 0.59 0.3361] Respawn Player
  (cast `/Game/BeginGame/GameMode/MyPlayerController` MyPlayerController)
  ;;[1 1 1] Do We Already Have a Pawn?
  (if (== _returnvalue null)
    ;;[1 1 1] Remove Pawn If required
    (`self.OutputLog` "We Have No Pawn")
    (else
      (`self.OutputLog` "We Have A Pawn")
      (`self.K2_DestroyActor` _returnvalue)))
  (`self.OutputLog` "I Choose Spawn : " (`KismetTextLibrary.Conv_TransformToText` _returnvalue_3))
  ;;[1 1 1] Spawn Actor For Possesion
  (bind _returnvalue_4 (`|SpawnActorFromClass` "/Game/BeginGame/Pawns/Basic_Pawn.Basic_Pawn_C" _returnvalue_3 "AlwaysSpawn" "OverrideRootScale" self))
  (`self.OutputLog` "Spawned Actor @ " (`KismetTextLibrary.Conv_IntToText` _returnvalue_2))
  (`self.ClientNumber` null)
  ;;[1 1 1] Posses the Actor From the MyPlayerController
  (`Controller.Possess` MyPlayerController _returnvalue_4))

(fn `ClientNumber`
  (params (PlayerController :type "/Game/BeginGame/GameMode/MyPlayerController Object Reference"))
  (for (_array_element _array_index) (`self.PlayerControllerRefs`)
    (if (== PlayerController _array_element)
      (`self.OutputLog` "Using Client number" (`KismetTextLibrary.Conv_IntToText` _array_index))))
  (return))

(fn `OutputLog`
  (params (text :type Text) (Test2 :type Text))
  (locals (Debug :type Boolean :default true))
  (if (`local.Debug`)
    (`KismetSystemLibrary.PrintText` (`|FormatText` "*GM_BeginGame {0} {1}" text Test2))))

(fn `UserConstructionScript`)